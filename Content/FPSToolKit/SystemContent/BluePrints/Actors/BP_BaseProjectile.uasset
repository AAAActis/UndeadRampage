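; Base projectile actor that deals point damage on hit, multiplied for "Head" bone hits, then destroys itself.
; Construction script feeds speed and ricochet settings into the ProjectileMovement component.
; Impact events pick particles and positional sound by physical material surface type, though the positional sound slots are unset.
; Body hits also play a 2D impact sound and notify the main HUD for hit feedback.
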(event Custom|Impact%20VFX%20Event
  (params (Hit :type Hit%20Result%20Structure%20%28by%20ref%29))
  (bind (_bblockinghit _binitialoverlap _time _distance _location _impactpoint _normal _impactnormal _physmat) (Collision|BreakHitResult Hit))
  ;[1 1 1] VFX per surface type
  (Utilities|IsValid _physmat
    (:Is%20Valid
      (Effects|SpawnEmitteratLocation (Utilities|Select :Index (Variables|/Script/PhysicsCore.PhysicalMaterial|GetSurfaceType _physmat) :SurfaceType_Default "/Game/FPSToolKit/DemoAssets/VFX/FX2/Particles/Abilities/Primary/FX/P_PlasmaShot_Hit_World.P_PlasmaShot_Hit_World" :SurfaceType1 "/Game/FPSToolKit/DemoAssets/VFX/FX2/Particles/Abilities/Primary/FX/P_PlasmaShot_Hit_Player.P_PlasmaShot_Hit_Player" :SurfaceType2 "/Game/FPSToolKit/DemoAssets/VFX/FX2/Particles/Abilities/Primary/FX/P_PlasmaShot_Hit_World.P_PlasmaShot_Hit_World" :SurfaceType3 0) _impactpoint (Math|Rotator|MakeRotfromX _impactnormal)))))

(event Custom|Impact%20SFX%20Event
  (params (Hit :type Hit%20Result%20Structure%20%28by%20ref%29))
  (bind (_bblockinghit _binitialoverlap _time _distance _location _impactpoint _normal _impactnormal _physmat) (Collision|BreakHitResult Hit))
  (bind _surfacetype (Variables|/Script/PhysicsCore.PhysicalMaterial|GetSurfaceType _physmat))
  ;[1 1 1] Sound per surface Type
  (Utilities|IsValid _physmat
    (:Is%20Valid
      (Audio|SpawnSoundatLocation (Utilities|Select :Index _surfacetype :SurfaceType_Default 0 :SurfaceType1 0 :SurfaceType2 0 :SurfaceType3 0) _impactpoint "0, 0, 0" 1.0 1.0 0.0 0 0)
      ;[1 1 1] Hit Feedback
      (switch Utilities|FlowControl|Switch|SwitchonEPhysicalSurface _surfacetype
        (:SurfaceType1
          (Audio|SpawnSound2D "/Game/FPSToolKit/DemoAssets/Sounds/Impact/SFX_BulletImpact_01_Cue.SFX_BulletImpact_01_Cue" 4.0 1.0 0.0 0)
          (Default|OnHitEvent (Variables|Default|GetMainHUD)))))))

(event EventBeginPlay)

(event Collision|EventActorBeginOverlap
  (params (OtherActor :type Actor%20Object%20Reference)))

(event EventTick
  (params (DeltaSeconds :type Float%20%28single-precision%29)))

(event Collision|EventHit
  (params (MyComp :type Primitive%20Component%20Object%20Reference) (Other :type Actor%20Object%20Reference) (OtherComp :type Primitive%20Component%20Object%20Reference) (bSelfMoved :type Boolean) (HitLocation :type Vector :default "0, 0, 0") (HitNormal :type Vector :default "0, 0, 0") (NormalImpulse :type Vector :default "0, 0, 0") (Hit :type Hit%20Result%20Structure%20%28by%20ref%29))
  (bind _damage (Variables|Default|GetDamage))
  ;[1 1 1] On hit apply point damage
  (Game|Damage|ApplyPointDamage Other (select (Utilities|Name|Equal(Name) (.HitBoneName (Collision|BreakHitResult Hit)) "Head") (* _damage (Variables|Default|GetDamageMultip)) _damage) (.TraceStart (Collision|BreakHitResult Hit)) Hit 0 (Components|GetOwner))
  (CallFunction|ImpactVFXEvent Hit)
  (CallFunction|ImpactSFXEvent Hit)
  (Actor|DestroyActor))

(fn ConstructionScript
  (bind _projectilemovement (Variables|Default|GetProjectileMovement))
  (bind _output_get (Variables|/Script/Engine.ProjectileMovementComponent|SetMaxSpeed _projectilemovement (Variables|Default|GetProjectile%20Speed)))
  (Variables|/Script/Engine.ProjectileMovementComponent|SetInitialSpeed _projectilemovement _output_get)
  (Variables|/Script/Engine.ProjectileMovementComponent|SetbShouldBounce _projectilemovement (Variables|Default|GetIs%20Ricochet)))