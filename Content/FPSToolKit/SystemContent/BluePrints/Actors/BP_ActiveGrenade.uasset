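; Thrown grenade actor for frag, smoke, molotov, proximity mine and flashbang types, configured on BeginPlay from DT_Grenades by GrenadeType.
; The first hit runs that type's behavior, with frag, smoke and flashbang delaying briefly unless they hit a projectile.
; Molotov and flashbang sphere-trace for victims to play reactions, and flashbang adds player post-process.
; Mines arm on impact, then hop on a looping timer and explode when a character or projectile overlaps.
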(event OnComponentBeginOverlap(MineTrigger)
  (params (OverlappedComponent :type Primitive%20Component%20Object%20Reference) (OtherActor :type Actor%20Object%20Reference) (OtherComp :type Primitive%20Component%20Object%20Reference) (OtherBodyIndex :type Integer) (bFromSweep :type Boolean) (SweepResult :type Hit%20Result%20Structure%20%28by%20ref%29))
  (|ActivateMine OtherActor))

(event Collision|EventActorBeginOverlap
  (params (OtherActor :type Actor%20Object%20Reference)))

(event EventTick
  (params (DeltaSeconds :type Float%20%28single-precision%29)))

(event EventBeginPlay
  ;[1 1 1] Comment
  (bind _outrownames (DataTable|GetDataTableRowNames "/Game/FPSToolKit/SystemContent/DataTables/DT_Grenades.DT_Grenades"))
  (for _array_element _outrownames
    (bind _returnvalue (Utilities|GetDataTableRow "/Game/FPSToolKit/SystemContent/DataTables/DT_Grenades.DT_Grenades" _array_element)
      (:then
        (if (Utilities|Enum|Equal(Enum) (Variables|DontTouch|GetGrenadeType) (.GrenadeType (Utilities|Struct|BreakF_Grenades _returnvalue)))
          (|SetGrenadeDetails (.Damage (Utilities|Struct|BreakF_Grenades _returnvalue)) (.DamageRadius (Utilities|Struct|BreakF_Grenades _returnvalue)) (.Mesh (Utilities|Struct|BreakF_Grenades _returnvalue)) (.CameraShake (Utilities|Struct|BreakF_Grenades _returnvalue)) (.CameraShakeScale (Utilities|Struct|BreakF_Grenades _returnvalue)) (.ExplosionSFX (Utilities|Struct|BreakF_Grenades _returnvalue)) (.ExplosionVFX (Utilities|Struct|BreakF_Grenades _returnvalue)) (.UseTrail (Utilities|Struct|BreakF_Grenades _returnvalue)) (.GrenadeTrail (Utilities|Struct|BreakF_Grenades _returnvalue))
            (:OutputPin
              (switch Utilities|FlowControl|Switch|SwitchonE_GrenadeType (Variables|DontTouch|GetGrenadeType)
                (:NewEnumerator3
                  (Components|Activation|Deactivate (Variables|Default|GetRotatingMovement)))))))))))

(event Collision|EventHit
  (params (MyComp :type Primitive%20Component%20Object%20Reference) (Other :type Actor%20Object%20Reference) (OtherComp :type Primitive%20Component%20Object%20Reference) (bSelfMoved :type Boolean) (HitLocation :type Vector :default "0, 0, 0") (HitNormal :type Vector :default "0, 0, 0") (NormalImpulse :type Vector :default "0, 0, 0") (Hit :type Hit%20Result%20Structure%20%28by%20ref%29))
  (Utilities|FlowControl|DoOnce false
    (:Completed
      (switch Utilities|FlowControl|Switch|SwitchonE_GrenadeType (Variables|DontTouch|GetGrenadeType)
        (:NewEnumerator0
          (|FragGrenade Other))
        (:NewEnumerator1
          (|SmokeGrenade Other))
        (:NewEnumerator2
          (|Molotov))
        (:NewEnumerator3
          (|Mine HitLocation))
        (:NewEnumerator5
          (|Flashbang Other))))))

(fn ConstructionScript)

(fn MineJump
  (Transformation|SetActorLocation (Math|Interpolation|VInterpTo (Transformation|GetActorLocation) (+ (Transformation|GetActorLocation) "0, 0,90.000000") (Utilities|Time|GetWorldDeltaSeconds) 4.0) false false))