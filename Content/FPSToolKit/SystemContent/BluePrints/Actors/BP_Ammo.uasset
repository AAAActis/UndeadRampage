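; BP_Ammo is an FPS ToolKit ammo pickup that supplies the current weapon, all weapons or a named weapon, depending on its AmmoType.
; On BeginPlay it fills its WBP_AmmoPickUp widget with type and amount, and tints the cube's outline through dynamic materials in a color per type.
; Trigger overlaps register or clear it as InteractedAmmo on the actor's AC_FPS_ToolKit and toggle the widget prompt, skipping the clear while grabbed.
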(event OnComponentBeginOverlap(InteractionTrigger)
  (params (OverlappedComponent :type Primitive%20Component%20Object%20Reference) (OtherActor :type Actor%20Object%20Reference) (OtherComp :type Primitive%20Component%20Object%20Reference) (OtherBodyIndex :type Integer) (bFromSweep :type Boolean) (SweepResult :type Hit%20Result%20Structure%20%28by%20ref%29))
  (bind _returnvalue (Actor|GetComponentbyClass OtherActor "/Game/FPSToolKit/SystemContent/BluePrints/AC_FPS_ToolKit.AC_FPS_ToolKit_C"))
  (Utilities|IsValid _returnvalue
    (:Is%20Valid
      (Variables|/Game/FPSToolKit/SystemContent/BluePrints/AC_FPS_ToolKit.AC_FPS_ToolKit_C|SetInteractedAmmo _returnvalue self)
      (Default|InteractionToggle (CallFunction|GetInfoWidget) true))))

(event OnComponentEndOverlap(InteractionTrigger)
  (params (OverlappedComponent :type Primitive%20Component%20Object%20Reference) (OtherActor :type Actor%20Object%20Reference) (OtherComp :type Primitive%20Component%20Object%20Reference) (OtherBodyIndex :type Integer))
  (bind _returnvalue (Actor|GetComponentbyClass OtherActor "/Game/FPSToolKit/SystemContent/BluePrints/AC_FPS_ToolKit.AC_FPS_ToolKit_C"))
  (bind _ammo_pick_up (CallFunction|GetInfoWidget))
  (if (not (Variables|Default|GetIsGrabbed))
    (Utilities|IsValid _returnvalue
      (:Is%20Valid
        (Variables|/Game/FPSToolKit/SystemContent/BluePrints/AC_FPS_ToolKit.AC_FPS_ToolKit_C|SetInteractedAmmo _returnvalue 0)
        (Utilities|IsValid _ammo_pick_up
          (:Is%20Valid
            (Default|InteractionToggle _ammo_pick_up false)))))))

(event EventBeginPlay
  (Default|SetAmmoInfo (CallFunction|GetInfoWidget) (Utilities|Select :Index (Variables|Default|GetAmmoType) :NewEnumerator0 "Current Weapon Ammo" :NewEnumerator1 "All Weapons Ammo" :NewEnumerator2 (Utilities|String|StringToName (Utilities|String|Append (Utilities|String|ToString(Name) (Variables|Default|GetWeaponName)) " Ammo"))) (Utilities|String|StringToName (Utilities|String|ToString(Integer) (Variables|Default|GetAmmoAmount))) (Utilities|Select :Index (Variables|Default|GetAmmoType) :NewEnumerator0 "(R=0.000000,G=0.246201,B=1.000000,A=1.000000)" :NewEnumerator1 "(R=0.684551,G=0.000000,B=1.000000,A=1.000000)" :NewEnumerator2 "(R=0.046665,G=0.381326,B=0.000000,A=1.000000)"))
  (for _array_element (Rendering|Material|GetMaterials (Variables|Default|GetCube))
    (bind _returnvalue (Rendering|Material|CreateDynamicMaterialInstance (Variables|Default|GetCube) 0 _array_element "None" :!class /Script/Engine.PrimitiveComponent))
    (Rendering|Material|SetVectorParameterValue _returnvalue "OutlineColor" (Utilities|Select :Index (Variables|Default|GetAmmoType) :NewEnumerator0 "(R=0.000000,G=0.246201,B=1.000000,A=1.000000)" :NewEnumerator1 "(R=0.684551,G=0.000000,B=1.000000,A=1.000000)" :NewEnumerator2 "(R=0.046665,G=0.381326,B=0.000000,A=1.000000)") :!class /Script/Engine.MaterialInstanceDynamic)))

(fn ConstructionScript)

(fn GetInfoWidget
  (return (.AsWBP%20Ammo%20Pick%20Up (Utilities|Casting|CastToWBP_AmmoPickUp (UserInterface|GetWidget (Variables|Default|GetWidget))))))