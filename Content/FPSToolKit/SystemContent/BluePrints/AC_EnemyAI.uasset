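; Enemy AI actor component for the FPS Toolkit that handles health, hit reactions and death on its owning character.
; DamageEvent subtracts health and triggers a front or back reaction montage, which blocks actions for most of its length.
; Radial reactions are limited to frag grenades and proximity mines.
; At zero health, the owner ragdolls with an impulse along the shot trace, and a headshot or kill sound plays.
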(event Custom|Play%20Hit%20Reaction%20Montage
  (params (IsRadialDamage :type Boolean) (DamageCauser :type Actor%20Object%20Reference))
  (bind _returnvalue (Components|GetOwner))
  (bind _returnvalue_2 (Actor|GetComponentbyClass _returnvalue "/Script/Engine.SkeletalMeshComponent"))
  (bind _returnvalue_3 (Components|SkeletalMesh|GetAnimInstance _returnvalue_2))
  (if IsRadialDamage
    (switch Utilities|FlowControl|Switch|SwitchonE_GrenadeType (Variables|/Game/FPSToolKit/SystemContent/BluePrints/AC_FPS_ToolKit.AC_FPS_ToolKit_C|GetGrenadeType (Actor|GetComponentbyClass DamageCauser "/Game/FPSToolKit/SystemContent/BluePrints/AC_FPS_ToolKit.AC_FPS_ToolKit_C"))
      (:NewEnumerator0
        _)
      (:NewEnumerator3
        _))
    (Utilities|IsValid _returnvalue_3
      (:Is%20Valid
        _)))
  (bind _returnvalue_4 (Animation|Montage|MontagePlay _returnvalue_3 (select (Utilities|IsFrontHit DamageCauser) (Variables|Default|GetFrontHitReaction) (Variables|Default|GetBackHitReaction)) 1.0 "MontageLength" 0.0 false))
  (Variables|Default|SetIsCantPerformAction true)
  (Utilities|FlowControl|Delay (* _returnvalue_4 0.8))
  (Variables|Default|SetIsCantPerformAction false))

(event Custom|Damage%20Event
  (params (Damage :type Float%20%28double-precision%29) (Hit%20Result :type Hit%20Result%20Structure) (DamageCauser :type Actor%20Object%20Reference))
  (if (Variables|Default|GetIsAlive)
    (bind _output_get (Variables|Default|SetHealth (- (Variables|Default|GetHealth) Damage)))
    (CallFunction|PlayHitReactionMontage false DamageCauser)
    (if (<= _output_get 0.0)
      (Variables|Default|SetIsAlive false)
      (CallFunction|Ragdoll Hit%20Result)
      (Audio|SpawnSound2D (select (Utilities|Name|Equal(Name) (.HitBoneName (Collision|BreakHitResult Hit%20Result)) (Variables|Default|GetHead%20Bone%20Name)) (Variables|Default|GetHeadShot) (Variables|Default|GetKill%20Sound)) 1.0 1.0 0.0 0))))

(event EventBeginPlay)

(event EventTick
  (params (DeltaSeconds :type Float%20%28single-precision%29)))

(fn Ragdoll
  (params (Hit%20Result :type Hit%20Result%20Structure))
  (bind _returnvalue (Components|GetOwner))
  (bind (_bblockinghit _binitialoverlap _time _distance _location _impactpoint _normal _impactnormal _physmat _hitactor _hitcomponent _hitbonename _bonename _hititem _elementindex _faceindex _tracestart _traceend) (Collision|BreakHitResult Hit%20Result))
  (bind _returnvalue_2 (Actor|GetComponentbyClass _returnvalue "/Script/Engine.SkeletalMeshComponent"))
  (bind _returnvalue_3 (Components|SkeletalMesh|GetAnimInstance _returnvalue_2))
  (Pawn|Components|CharacterMovement|SetMovementMode (Actor|GetComponentbyClass _returnvalue "/Script/Engine.CharacterMovementComponent") "MOVE_None" 0)
  (Collision|SetCollisionEnabled (Actor|GetComponentbyClass _returnvalue "/Script/Engine.CapsuleComponent") "NoCollision")
  (Collision|SetCollisionObjectType _returnvalue_2 "ECC_PhysicsBody")
  (Collision|SetCollisionEnabled _returnvalue_2 "QueryAndPhysics")
  (Physics|SetSimulatePhysics _returnvalue_2 true)
  (Utilities|IsValid _returnvalue_3
    (:Is%20Valid
      (Animation|Montage|MontageStop _returnvalue_3 0.25 0)
      (Physics|AddImpulseatLocation (Actor|GetComponentbyClass (Components|GetOwner) "/Script/Engine.SkeletalMeshComponent") (* (- _traceend _tracestart) 3e+01) _impactpoint _hitbonename))))